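; AIBot is an AI controller that drives a possessed Bot pawn through a behavior tree.
; On possess it sets up the attack blackboard, seeds it with the bot's health and current waypoint as target, then runs BotTree.
; A helper writes the EnemicTrobat (enemy found) flag to the blackboard.
; The DeteccioEnemic detection function is an empty stub, and the raycast clock is only initialized here.
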(event `self.OnPossess`
  (params (PossessedPawn :type "Pawn Object Reference"))
  (`self.Initialize`)
  (set `self.Clock` (`self.Raycasting_Frequency`))
  (`self.RunBehaviorTree` "/Game/BluePrints/IA/BotTree.BotTree"))

(fn `ActualitzarBlackboard_EnemicTrobat`
  (params (EnemicTrobat :type Boolean))
  (`BlackboardComponent.SetValueAsBool` (`AIBlueprintHelperLibrary.GetBlackboard` self) "EnemicTrobat" EnemicTrobat)
  (return))

(fn `DeteccioEnemic`)

(fn `Initialize`
  (bind _returnvalue (`AIBlueprintHelperLibrary.GetBlackboard` self))
  (`self.UseBlackboard` "/Game/BluePrints/IA/AttackBotBlackboard.AttackBotBlackboard")
  (bind _asbot (cast `/Game/Assets/3DModels/Bot` (`self.K2_GetPawn`)))
  (set `self.Controlat` _asbot)
  (`BlackboardComponent.SetValueAsFloat` _returnvalue "CurrentHealth" (`/Game/Assets/3DModels/Bot.Health` _asbot))
  (bind _waypointpos (`/Game/Assets/3DModels/Bot.GetCurrentWaypoint` (`self.Controlat`)))
  (`BlackboardComponent.SetValueAsVector` _returnvalue "Target" _waypointpos)
  (return))

(fn `UserConstructionScript`)